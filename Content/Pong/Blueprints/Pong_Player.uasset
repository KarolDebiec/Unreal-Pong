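; Pong player Blueprint that runs a local match, moving both paddles and managing the ball, countdown timer and game screens.
; BeginPlay shows the StartGame widget and spawns a waiting ball, which D or V launches with a random impulse once starting is allowed.
; Tick polls keys to slide both paddles within X borders, and switches to the EndGame widget when either score hits MaxScore or time expires.
; Separate events respawn balls and reset the timer.
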(event `Event NextBallResp`
  (bind _returnvalue (`|SpawnActorFromClass` "/Game/Pong/Blueprints/Ball.Ball_C" (`KismetMathLibrary.MakeTransform` (0.0 -600.0 30.0) (struct) (0.8 0.8 0.8)) "Undefined" "OverrideRootScale" null null))
  (`/Game/Pong/Blueprints/Ball.Random Impulse Ball` _returnvalue))

(event `RestartBall`
  (bind _returnvalue (`|SpawnActorFromClass` "/Game/Pong/Blueprints/Ball.Ball_C" (`KismetMathLibrary.MakeTransform` (0.0 -600.0 30.0) (struct) (0.8 0.8 0.8)) "Undefined" "OverrideRootScale" null null :!label _label)))

(event `self.ReceiveBeginPlay`
  (bind _returnvalue (`|CreateWidget` "/Game/Pong/Blueprints/StartGame.StartGame_C"))
  (`UserWidget.AddToViewport` _returnvalue 0)
  (goto _label))

(event `self.ReceiveTick`
  (params (DeltaSeconds :type "Float (single-precision)"))
  (bind _movingspeed (`self.movingSpeed`))
  (bind _enemycube (`self.EnemyCube`))
  (bind _movingspeed_2 (`self.movingSpeed`))
  (bind _cube (`self.Cube`))
  (bind _returnvalue_x (`KismetMathLibrary.BreakVector` (`SceneComponent.K2_GetComponentLocation` _cube)))
  (bind _returnvalue_x_2 (`KismetMathLibrary.BreakVector` (`SceneComponent.K2_GetComponentLocation` _cube)))
  (bind _returnvalue_x_3 (`KismetMathLibrary.BreakVector` (`SceneComponent.K2_GetComponentLocation` _enemycube)))
  (bind _returnvalue_x_4 (`KismetMathLibrary.BreakVector` (`SceneComponent.K2_GetComponentLocation` _enemycube)))
  (if (`self.isGameStarted`)
    (bind _output_get (set `self.timer` (- (`self.timer`) DeltaSeconds)))
    (if (<= (`self.maxScore`) (`self.scoreLeft`))
      (set `self.isGameStarted` false :!label _label_2)
      (set `self.timer` 0.0)
      (`WidgetLayoutLibrary.RemoveAllWidgets`)
      (bind _returnvalue (`|CreateWidget` "/Game/Pong/Blueprints/EndGame.EndGame_C"))
      (`Widget.ResetCursor` _returnvalue)
      (`UserWidget.AddToViewport` _returnvalue 0)
      (`Widget.SetCursor` _returnvalue "Default")
      (`self.K2_DestroyActor` (stale `Event NextBallResp` _returnvalue))
      (elif (<= (`self.maxScore`) (`self.scoreRight`))
        (goto _label_2)
        (elif (< _output_get 0.0)
          (goto _label_2)
          (else
            ;[1 1 1] Ruch lewej paletki ograniczony wpisanymi maksymalnymi dopuszczalnymi granicami poruszania sie po osi x
            (if (`PlayerController.IsInputKeyDown` (`GameplayStatics.GetPlayerController` 0) (stale `Key|D` Key))
              (if (< _returnvalue_x (`self.enemyUpBorder`))
                (`SceneComponent.K2_AddLocalOffset` _cube (`KismetMathLibrary.MakeVector` (* DeltaSeconds _movingspeed)) false false))
              (elif (`PlayerController.IsInputKeyDown` (`GameplayStatics.GetPlayerController` 0) (stale `Key|V` Key))
                (if (< (`self.enemyDownBorder`) _returnvalue_x_2)
                  (`SceneComponent.K2_AddLocalOffset` _cube (`KismetMathLibrary.MakeVector` (* DeltaSeconds (* -1.0 _movingspeed))) false false))))
            ;[1 1 1] Ruch prawej paletki ograniczony wpisanymi maksymalnymi dopuszczalnymi granicami poruszania sie po osi x
            (if (`PlayerController.IsInputKeyDown` (`GameplayStatics.GetPlayerController` 0) (stale `Key|Up` Key)) :!label _label_3
              (if (< _returnvalue_x_3 (`self.enemyUpBorder`))
                (`SceneComponent.K2_AddLocalOffset` _enemycube (`KismetMathLibrary.MakeVector` (* DeltaSeconds _movingspeed_2)) false false))
              (else
                (if (`PlayerController.IsInputKeyDown` (`GameplayStatics.GetPlayerController` 0) (stale `Key|Left` Key)) :!label _label_4
                  (if (< (`self.enemyDownBorder`) _returnvalue_x_4)
                    (`SceneComponent.K2_AddLocalOffset` _enemycube (`KismetMathLibrary.MakeVector` (* DeltaSeconds (* -1.0 _movingspeed_2))) false false)))))))))))

(event `Key|Up`
  (params (Key :type "Key Structure"))
  ;[1 1 1] Ruch prawej paletki ograniczony wpisanymi maksymalnymi dopuszczalnymi granicami poruszania sie po osi x
  (:`Pressed`
    (goto _label_3)))

(event `Key|D`
  (params (Key :type "Key Structure"))
  (:`Pressed`
    (if (`self.canStartGame`) :!label _label_5
      (if (not (`self.isGameStarted`))
        (set `self.canStartGame` false)
        (set `self.isGameStarted` true)
        (`/Game/Pong/Blueprints/Ball.Random Impulse Ball` (stale `RestartBall` _returnvalue))))))

(event `Key|Left`
  (params (Key :type "Key Structure"))
  ;[1 1 1] Ruch prawej paletki ograniczony wpisanymi maksymalnymi dopuszczalnymi granicami poruszania sie po osi x
  (:`Pressed`
    (goto _label_4)))

(event `Key|V`
  (params (Key :type "Key Structure"))
  (:`Pressed`
    (goto _label_5)))

(fn `ResetTimer`
  (set `self.timer` (`self.timeLimit`)))

(fn `UserConstructionScript`)